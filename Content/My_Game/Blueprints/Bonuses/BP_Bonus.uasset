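; BP_Bonus is a bonus actor that randomly becomes one of three types, MAX, LIVE or BALL, and travels through the level.
; The construction script rolls the type and gives the cylinder a matching turquoise, violet or red material.
; Each tick moves the actor with sweep along world X only, scaled by Direction, Speed and delta time.
; The graphs contain no pickup or effect logic.
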(event `self.ReceiveTick`
  (params (DeltaSeconds :type "Float (single-precision)"))
  (bind _returnvalue_x (`KismetMathLibrary.BreakVector` (* (`self.Direction`) (* DeltaSeconds (`self.Speed`)))))
  (`self.K2_AddActorWorldOffset` (`KismetMathLibrary.MakeVector` _returnvalue_x) true))

(fn `UserConstructionScript`
  (bind _cylinder (`self.Cylinder`))
  (bind _output_get (set `self.BonusType` (select `int` (`KismetMathLibrary.RandomIntegerInRange` 0 2) :`0` "NewEnumerator0" :`1` "NewEnumerator1" :`2` "NewEnumerator2" :!type "/Game/My_Game/Blueprints/Bonuses/E_Bonus_Type Enum")))
  (switch `/Game/My_Game/Blueprints/Bonuses/E_Bonus_Type` _output_get
    (:`NewEnumerator0`
      (`PrimitiveComponent.SetMaterial` _cylinder 0 "/Game/My_Game/Materials/MI_Color_Turquoise.MI_Color_Turquoise"))
    (:`NewEnumerator1`
      (`PrimitiveComponent.SetMaterial` _cylinder 0 "/Game/My_Game/Materials/MI_Color_Violet.MI_Color_Violet"))
    (:`NewEnumerator2`
      (`PrimitiveComponent.SetMaterial` _cylinder 0 "/Game/My_Game/Materials/MI_Color_Red.MI_Color_Red"))))