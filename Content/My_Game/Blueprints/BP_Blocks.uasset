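; BP_Blocks is a grid placer that spawns a flat array of BP_Cube_Child actors when play begins.
; The construction script adds static mesh components in a grid sized by X and Y and spaced by Padding, storing them in PreviewArray as a preview.
; BeginPlay destroys those preview components, then spawns the cube actors at matching offsets from the actor's location along world X and Y.
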(event `self.ReceiveBeginPlay`
  (bind (_returnvalue_x _returnvalue_y _returnvalue_z) (`KismetMathLibrary.BreakVector` (`self.K2_GetActorLocation`)))
  (for _array_element (`self.PreviewArray`)
    (`ActorComponent.K2_DestroyComponent` _array_element))
  (for _index (range (+ (`self.X`) 1))
    (for _index_2 (range (+ (`self.Y`) 1))
      (`|SpawnActorFromClass` "/Game/My_Game/Blueprints/BP_Cube_Child.BP_Cube_Child_C" (`KismetMathLibrary.MakeTransform` (`KismetMathLibrary.MakeVector` (+ _returnvalue_x (`KismetMathLibrary.Conv_IntToDouble` (* _index (`self.Padding`)))) (+ _returnvalue_y (`KismetMathLibrary.Conv_IntToDouble` (* _index_2 (`self.Padding`)))) _returnvalue_z)) "Undefined" "OverrideRootScale" null null))))

(fn `UserConstructionScript`
  (for _index (range (+ (`self.X`) 1))
    (for _index_2 (range (+ (`self.Y`) 1))
      (bind _returnvalue (`AddComponent|NODE_AddStaticMeshComponent-0` :`RelativeTransform` (`KismetMathLibrary.MakeTransform` (`KismetMathLibrary.MakeVector` (`KismetMathLibrary.Conv_IntToDouble` (* _index (`self.Padding`))) (`KismetMathLibrary.Conv_IntToDouble` (* _index_2 (`self.Padding`)))))))
      (`KismetArrayLibrary.Array_Add` (`self.PreviewArray`) _returnvalue))))