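; BP_Cube_Child is a child cube Blueprint that can drop a bonus pickup when destroyed.
; On BeginPlay it binds to OnDestroyed only if the cube's first material is MI_Metal_Gold, so the material marks bonus cubes.
; The bound event spawns BP_Bonus at the cube's location with a fixed rotation, ignoring collisions.
; BallIsHit and the construction script only call their parent versions.
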(event `self.ReceiveBeginPlay`
  (if (== (`PrimitiveComponent.GetMaterial` (`self.Cube`) 0) "/Game/My_Game/Materials/Metals/MI_Metal_Gold.MI_Metal_Gold")
    (add `self.OnDestroyed` (delegate `SpawnBonus`))))

(event `SpawnBonus`
  (params (DestroyedActor :type "Actor Object Reference"))
  (`|SpawnActorFromClass` "/Game/My_Game/Blueprints/Bonuses/BP_Bonus.BP_Bonus_C" (`KismetMathLibrary.MakeTransform` (`self.K2_GetActorLocation`) (struct :`Pitch` -90.0)) "AlwaysSpawn" "OverrideRootScale" null null))

(event `self.BallIsHit`
  (`parent.BallIsHit`))

(fn `UserConstructionScript`
  (`parent.UserConstructionScript`))