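; BP_My_PlayerController is the player controller that turns input into movement and ball spawning for BP_My_Pawn.
; On possession it casts and caches the pawn, and on BeginPlay it switches input to game-only.
; The Left_Right axis slides the pawn along world Y with a swept, delta-time-scaled offset based on Speed.
; The SpawnBall action forwards to the pawn's own SpawnBall function.
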(event `self.ReceiveBeginPlay`
  (`WidgetBlueprintLibrary.SetInputMode_GameOnly` self))

(event `self.ReceivePossess`
  (params (PossessedPawn :type "Pawn Object Reference"))
  (bind _asbp_my_pawn (cast `/Game/My_Game/Blueprints/Core/BP_My_Pawn` PossessedPawn))
  (set `self.MyPawn ` _asbp_my_pawn))

(event `InputAxis|Left_Right`
  (params (AxisValue :type "Float (single-precision)"))
  (`self.K2_AddActorWorldOffset` (`self.MyPawn `) (`KismetMathLibrary.MakeVector` 0.0 (* AxisValue (`GameplayStatics.GetWorldDeltaSeconds`) (`self.Speed`))) true false))

(event `InputAction|SpawnBall`
  (params (Key :type "Key Structure"))
  (:`Pressed`
    (`/Game/My_Game/Blueprints/Core/BP_My_Pawn.SpawnBall` (`self.MyPawn `))))

(fn `UserConstructionScript`)