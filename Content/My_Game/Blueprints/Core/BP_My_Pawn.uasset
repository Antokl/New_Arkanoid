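; Player paddle pawn for what appears to be a Breakout-style game, handling ball spawning, lives and bonus pickups.
; SpawnBall launches a ball from the Arrow while lives remain and none is alive; its destruction costs a life or prints Game Over.
; Cube overlaps dispatch BP_Bonus types: temporary widening reset by a retriggerable delay, an extra life, or a smaller untracked extra ball.
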(event `self.ReceiveBeginPlay`
  (set `self.DefaultScale` (`SceneComponent.RelativeScale3D` (`self.Cube`))))

(event `SpawnBall`
  (if (not (<= (`self.PlayerLives`) 0))
    (`self.AliveBall`
      (:`then`)
      (:`else`
        (bind _returnvalue (`|SpawnActorFromClass` "/Game/My_Game/Blueprints/BP_Ball.BP_Ball_C" (`KismetMathLibrary.MakeTransform` (`SceneComponent.K2_GetComponentLocation` (`self.Arrow`))) "Undefined" "OverrideRootScale" null null))
        (bind _output_get (set `self.AliveBall` _returnvalue))
        (add `self.OnDestroyed` _output_get (delegate `BallIsDead`))
        (`SceneComponent.SetVisibility` (`self.TextRender`) false false)))))

(event `BallIsDead` :!signature `self.OnDestroyed`
  (params (DestroyedActor :type "Actor Object Reference"))
  (bind _result (`/Engine/EditorBlueprintResources/StandardMacros.DecrementInt` (`self.PlayerLives`))
    (:`  `
      (if (<= _result 0)
        (`KismetSystemLibrary.PrintString` "Game Over" true true (struct :`R` 1.0 :`G` 0.015526 :`A` 1.0))
        (else
          (`SceneComponent.SetVisibility` (`self.TextRender`) false false)
          (`GameplayStatics.PlaySoundAtLocation` "/Game/My_Game/Sounds/VR_close_Dead.VR_close_Dead" (`self.K2_GetActorLocation`) (struct) 1.0 1.0 0.0 null null null))))))

(event `self.Cube.OnComponentBeginOverlap`
  (params (OverlappedComponent :type "PrimitiveComponent Object Reference") (OtherActor :type "Actor Object Reference") (OtherComp :type "PrimitiveComponent Object Reference") (OtherBodyIndex :type Integer) (bFromSweep :type Boolean) (SweepResult :type "HitResult Structure (by ref)"))
  (bind _asbp_bonus (cast `/Game/My_Game/Blueprints/Bonuses/BP_Bonus` OtherActor))
  (switch `/Game/My_Game/Blueprints/Bonuses/E_Bonus_Type` (`/Game/My_Game/Blueprints/Bonuses/BP_Bonus.BonusType` _asbp_bonus)
    (:`NewEnumerator0`
      (`self.MaxEvent`))
    (:`NewEnumerator1`
      (`self.LiveEvent`))
    (:`NewEnumerator2`
      (`self.BallEvent`)))
  (`GameplayStatics.PlaySoundAtLocation` "/Game/My_Game/Sounds/VR_close_Bonus.VR_close_Bonus" (`self.K2_GetActorLocation`) (struct) 1.0 1.0 0.0 null null null)
  (`self.K2_DestroyActor` _asbp_bonus))

(event `MaxEvent`
  (bind _cube (`self.Cube`))
  (bind (_relativescale3d_x _relativescale3d_y _relativescale3d_z) (`KismetMathLibrary.BreakVector` (`SceneComponent.RelativeScale3D` _cube)))
  (`SceneComponent.SetRelativeScale3D` _cube (`KismetMathLibrary.MakeVector` _relativescale3d_x (* _relativescale3d_y 1.2) _relativescale3d_z))
  (`self.MinEvent`))

(event `MinEvent`
  (`KismetSystemLibrary.RetriggerableDelay` 5.0)
  (`SceneComponent.SetRelativeScale3D` (`self.Cube`) (`self.DefaultScale`)))

(event `LiveEvent`
  (bind _result (`/Engine/EditorBlueprintResources/StandardMacros.IncrementInt` (`self.PlayerLives`))
    (:`  `
      (`KismetSystemLibrary.PrintString` (`KismetStringLibrary.Conv_IntToString` _result) true true (struct :`R` 1.0 :`G` 0.038955 :`A` 1.0) 7.0)
      (`KismetSystemLibrary.PrintString` "Live" true true (struct :`R` 1.0 :`G` 0.009744 :`A` 1.0) 7.0))))

(event `BallEvent`
  (`|SpawnActorFromClass` "/Game/My_Game/Blueprints/BP_Ball.BP_Ball_C" (`KismetMathLibrary.MakeTransform` (`SceneComponent.K2_GetComponentLocation` (`self.Arrow`)) (struct) (0.7 0.7 0.7)) "Undefined" "OverrideRootScale" null null))

(fn `UserConstructionScript`)